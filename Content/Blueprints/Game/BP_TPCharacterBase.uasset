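; Base third-person character Blueprint that drives dynamic camera framing for running and aiming, with weapon-aware adjustments.
; BeginPlay caches camera and spring arm defaults and binds a still-empty aim input handler.
; Tick eases FOV and arm length with FInterpTo, pulling in for armed aiming and widening for forward running, less so when armed.
; Tick also prints input-state debug text, while spine-socket camera attachment and aim turn montages sit disconnected.
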(event Custom|AimInputTrigger_Event
  (params (bAim :type Boolean)))

(event Custom|Debug
  (Development|PrintString (Utilities|String|Append "MoveAxis:" (Utilities|String|ToString(Vector2d) (Variables|Default|GetMoveAxis))) true true "(R=0.000000,G=0.660000,B=1.000000,A=1.000000)" 0.0)
  (Development|PrintString (Utilities|String|Append "bRun:" (Utilities|String|ToString(Boolean) (Variables|Default|GetbRun))) true true "(R=0.000000,G=0.660000,B=1.000000,A=1.000000)" 0.0)
  (Development|PrintString (Utilities|String|Append "bMoveX:" (Utilities|String|ToString(Boolean) (Variables|Default|GetbMoveInputX)) "   " "bMoveY:" (Utilities|String|ToString(Boolean) (Variables|Default|GetbMoveInputY))) true true "(R=1.000000,G=0.493314,B=0.058804,A=1.000000)" 0.0)
  (Development|PrintString (Utilities|String|Append "bAim:" (Utilities|String|ToString(Boolean) (Variables|Default|GetbAim))) true true "(R=1.000000,G=0.493314,B=0.058804,A=1.000000)" 0.0)
  (Development|PrintString (Utilities|String|Append "bPackUp:" (Utilities|String|ToString(Boolean) (Variables|Default|GetbPackUp))) true true "(R=0.115493,G=0.000000,B=1.000000,A=1.000000)" 0.0)
  (Development|PrintString (Utilities|String|Append "bEquip:" (Utilities|String|ToString(Boolean) (Variables|Default|GetbEquip))) true true "(R=0.000000,G=0.618336,B=1.000000,A=1.000000)" 0.0))

(event EventTick
  (params (DeltaSeconds :type Float%20%28single-precision%29))
  (Utilities|FlowControl|Sequence
    (:then_0
      (CallFunction|UpdateFOV 1.5 1e+01 1e+01 -3e+01)
      (CallFunction|UpdateTargetArmLength 1.5 3e+01 1e+01 -2e+01))
    (:then_1
      (CallFunction|Debug))))

(event EventBeginPlay
  (bind _output_get (Variables|Camera|SetBaseFOV (Variables|/Script/Engine.CameraComponent|GetFieldOfView (Variables|Default|GetPlayerCameraComp))))
  (Variables|Camera|SetCurrentFOV _output_get)
  (bind _output_get_2 (Variables|Camera|SetBaseTargetArmLength (Variables|/Script/Engine.SpringArmComponent|GetTargetArmLength (Variables|Default|GetPlayerCameraSpringArmComp))))
  (Variables|Camera|SetCurrentTargetArmLength _output_get_2)
  (Variables|Camera|SetBaseSocketOffset (Variables|/Script/Engine.SpringArmComponent|GetSocketOffset (Variables|Default|GetPlayerCameraSpringArmComp)))
  (EventDispatchers|AssignAimInputTrigger (delegate Custom|AimInputTrigger_Event)))

(fn ConstructionScript)

(fn UpdateFOV
  (params (RunSpeed :type Float%20%28double-precision%29) (RunFOV :type Float%20%28double-precision%29) (AimFOVSpeed :type Float%20%28double-precision%29) (AimFOV :type Float%20%28double-precision%29))
  (LocalVariables|SetLocal_RunFOVSpeed RunSpeed)
  (LocalVariables|SetLocal_RunFOV RunFOV)
  (LocalVariables|SetLocal_AimFOVSpeed AimFOVSpeed)
  (LocalVariables|SetLocal_AimFOV AimFOV)
  (Utilities|FlowControl|Sequence
    (:then_0
      (if (and (Variables|Default|GetbAim) (Utilities|IsValid (Variables|Default|GetCurrentWeapon)))
        (LocalVariables|SetTargetFOV (+ (Variables|Camera|GetBaseFOV) (LocalVariables|GetLocal_AimFOV)))
        (LocalVariables|SetTargetSpeed (LocalVariables|GetLocal_AimFOVSpeed))
        (elif (< (+ (Variables|Camera|GetCurrentFOV) 1.0) (Variables|Camera|GetBaseFOV))
          (LocalVariables|SetTargetFOV (Variables|Camera|GetBaseFOV))
          (LocalVariables|SetTargetSpeed (LocalVariables|GetLocal_AimFOVSpeed))
          (elif (> (.y (Variables|Default|GetMoveAxis)) 0.001)
            (if (Variables|Default|GetbRun)
              (LocalVariables|SetTargetFOV (+ (Variables|Camera|GetBaseFOV) (LocalVariables|GetLocal_RunFOV)))
              (LocalVariables|SetTargetSpeed (LocalVariables|GetLocal_RunFOVSpeed))
              (if (Utilities|IsValid (Variables|Default|GetCurrentWeapon))
                (LocalVariables|SetTargetFOV (+ (Variables|Camera|GetBaseFOV) (/ (LocalVariables|GetLocal_RunFOV) 1.5))))
              (else
                (LocalVariables|SetTargetFOV (Variables|Camera|GetBaseFOV) :!label _label)
                (LocalVariables|SetTargetSpeed (LocalVariables|GetLocal_RunFOVSpeed))))
            (else
              (goto _label))))))
    (:then_2
      (if (not (Math|Float|NearlyEqual(Float) (Variables|Camera|GetCurrentFOV) (LocalVariables|GetTargetFOV) 0.001))
        (Variables|Camera|SetCurrentFOV (Math|Interpolation|FInterpTo (Variables|Camera|GetCurrentFOV) (LocalVariables|GetTargetFOV) (Utilities|Time|GetWorldDeltaSeconds) (LocalVariables|GetTargetSpeed)))
        (Camera|SetFieldOfView (Variables|Default|GetPlayerCameraComp) (Variables|Camera|GetCurrentFOV))))))

(fn UpdateTargetArmLength
  (params (RunBeginSpeed :type Float%20%28double-precision%29) (RunValue :type Float%20%28double-precision%29) (AimSpeed :type Float%20%28double-precision%29) (AimValue :type Float%20%28double-precision%29))
  (LocalVariables|SetLocal_RunSpeed RunBeginSpeed)
  (LocalVariables|SetLocal_RunValue RunValue)
  (LocalVariables|SetLocal_AimValue AimValue)
  (LocalVariables|SetLocal_AimSpeed AimSpeed)
  (Utilities|FlowControl|Sequence
    (:then_0
      (if (and (Variables|Default|GetbAim) (Utilities|IsValid (Variables|Default|GetCurrentWeapon)))
        (LocalVariables|SetTarget (+ (Variables|Camera|GetBaseTargetArmLength) (LocalVariables|GetLocal_AimValue)))
        (LocalVariables|SetSpeed (LocalVariables|GetLocal_AimSpeed))
        (elif (< (+ (Variables|Camera|GetCurrentTargetArmLength) 2.0) (Variables|Camera|GetBaseTargetArmLength))
          (LocalVariables|SetTarget (Variables|Camera|GetBaseTargetArmLength))
          (LocalVariables|SetSpeed (LocalVariables|GetLocal_AimSpeed))
          (elif (> (.y (Variables|Default|GetMoveAxis)) 0.001)
            (if (Variables|Default|GetbRun)
              (LocalVariables|SetTarget (+ (Variables|Camera|GetBaseTargetArmLength) (LocalVariables|GetLocal_RunValue)))
              (LocalVariables|SetSpeed (LocalVariables|GetLocal_RunSpeed))
              (if (Utilities|IsValid (Variables|Default|GetCurrentWeapon))
                (LocalVariables|SetTarget (+ (Variables|Camera|GetBaseTargetArmLength) (/ (LocalVariables|GetLocal_RunValue) 2.5))))
              (else
                (LocalVariables|SetTarget (Variables|Camera|GetBaseTargetArmLength) :!label _label)
                (LocalVariables|SetSpeed (LocalVariables|GetLocal_RunSpeed))))
            (else
              (goto _label))))))
    (:then_1
      (if (not (Math|Float|NearlyEqual(Float) (Variables|Camera|GetCurrentTargetArmLength) (LocalVariables|GetTarget) 0.1))
        (bind _output_get (Variables|Camera|SetCurrentTargetArmLength (Math|Interpolation|FInterpTo (Variables|Camera|GetCurrentTargetArmLength) (LocalVariables|GetTarget) (Utilities|Time|GetWorldDeltaSeconds) (LocalVariables|GetSpeed))))
        (Variables|/Script/Engine.SpringArmComponent|SetTargetArmLength (Variables|Default|GetPlayerCameraSpringArmComp) _output_get)))))