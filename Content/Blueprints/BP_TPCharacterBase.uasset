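; Third-person character base Blueprint that drives a run camera effect and records the camera's default FOV and spring arm length at BeginPlay.
; Each tick, running forward eases FOV narrower and the arm longer, a dolly-zoom-style effect, otherwise both ease back to defaults.
; Separate interpolation speeds govern entering and leaving the effect.
; Tick also prints move axis, run and input flags for debugging.
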(event Custom|Debug
  (Development|PrintString (Utilities|String|Append "MoveAxis:" (Utilities|String|ToString(Vector2d) (Variables|Default|Get_moveAxis))) true true "(R=0.000000,G=0.660000,B=1.000000,A=1.000000)" 0.0)
  (Development|PrintString (Utilities|String|Append "bRun:" (Utilities|String|ToString(Boolean) (Variables|Default|Get_bRun))) true true "(R=0.000000,G=0.660000,B=1.000000,A=1.000000)" 0.0)
  (Development|PrintString (Utilities|String|Append "bMoveX:" (Utilities|String|ToString(Boolean) (Variables|Default|Get_bMoveInputX)) "   " "bMoveY:" (Utilities|String|ToString(Boolean) (Variables|Default|Get_bMoveInputY))) true true "(R=1.000000,G=0.493314,B=0.058804,A=1.000000)" 0.0))

(event EventBeginPlay
  (bind _output_get (Variables|Camera|SetBaseFOV (Variables|/Script/Engine.CameraComponent|GetFieldOfView (Variables|Default|Get_playerCameraComp))))
  (Variables|Camera|SetCurrentFOV _output_get)
  (bind _output_get_2 (Variables|Camera|SetBaseTargetArmLength (Variables|/Script/Engine.SpringArmComponent|GetTargetArmLength (Variables|Default|Get_playerCameraSpringArmComp))))
  (Variables|Camera|SetCurrentTargetArmLength _output_get_2))

(event Collision|EventActorBeginOverlap
  (params (OtherActor :type Actor%20Object%20Reference)))

(event EventTick
  (params (DeltaSeconds :type Float%20%28single-precision%29))
  (Utilities|FlowControl|Sequence
    (:then_0
      (CallFunction|UpdateFOV 2.0 3.5 -15.0)
      (CallFunction|UpdateTargetArmLength 1.0 2.5 1e+02))
    (:then_1
      (CallFunction|Debug))))

(fn ConstructionScript)

(fn UpdateFOV
  (params (RunBeginSpeed :type Float%20%28double-precision%29) (RunEndSpeed :type Float%20%28double-precision%29) (RunFOV :type Float%20%28double-precision%29))
  (LocalVariables|SetLocal_RunFOVBeginSpeed RunBeginSpeed)
  (LocalVariables|SetLocal_RunFOVEndSpeed RunEndSpeed)
  (LocalVariables|SetLocal_RunFOV RunFOV)
  (Utilities|FlowControl|Sequence
    (:then_0
      (if (> (Math|Vector|DotProduct (Transformation|GetActorForwardVector) (Variables|/Script/Engine.MovementComponent|GetVelocity (Variables|Character|GetCharacterMovement))) 1e+01)
        (if (Variables|Default|Get_bRun)
          (Variables|Camera|SetCurrentFOV (Math|Interpolation|FInterpTo (Variables|Camera|GetCurrentFOV) (+ (Variables|Camera|GetBaseFOV) (LocalVariables|GetLocal_RunFOV)) (Utilities|Time|GetWorldDeltaSeconds) (LocalVariables|GetLocal_RunFOVBeginSpeed)))
          (else
            (Variables|Camera|SetCurrentFOV (Math|Interpolation|FInterpTo (Variables|Camera|GetCurrentFOV) (Variables|Camera|GetBaseFOV) (Utilities|Time|GetWorldDeltaSeconds) (LocalVariables|GetLocal_RunFOVEndSpeed)) :!label _label)))
        (else
          (goto _label))))
    (:then_2
      (Camera|SetFieldOfView (Variables|Default|Get_playerCameraComp) (Variables|Camera|GetCurrentFOV)))))

(fn UpdateTargetArmLength
  (params (RunBeginSpeed :type Float%20%28double-precision%29) (RunEndSpeed :type Float%20%28double-precision%29) (RunValue :type Float%20%28double-precision%29))
  (LocalVariables|SetLocal_RunBeginSpeed RunBeginSpeed)
  (LocalVariables|SetLocal_RunEndSpeed RunEndSpeed)
  (LocalVariables|SetLocal_RunValue RunValue)
  (Utilities|FlowControl|Sequence
    (:then_0
      (if (> (Math|Vector|DotProduct (Transformation|GetActorForwardVector) (Variables|/Script/Engine.MovementComponent|GetVelocity (Variables|Character|GetCharacterMovement))) 1e+01)
        (if (Variables|Default|Get_bRun)
          (Variables|Camera|SetCurrentTargetArmLength (Math|Interpolation|FInterpTo (Variables|Camera|GetCurrentTargetArmLength) (+ (Variables|Camera|GetBaseTargetArmLength) (LocalVariables|GetLocal_RunValue)) (Utilities|Time|GetWorldDeltaSeconds) (LocalVariables|GetLocal_RunBeginSpeed)))
          (else
            (Variables|Camera|SetCurrentTargetArmLength (Math|Interpolation|FInterpTo (Variables|Camera|GetCurrentTargetArmLength) (Variables|Camera|GetBaseTargetArmLength) (Utilities|Time|GetWorldDeltaSeconds) (LocalVariables|GetLocal_RunEndSpeed)) :!label _label)))
        (else
          (goto _label))))
    (:then_2
      (Variables|/Script/Engine.SpringArmComponent|SetTargetArmLength (Variables|Default|Get_playerCameraSpringArmComp) (Variables|Camera|GetCurrentTargetArmLength)))))